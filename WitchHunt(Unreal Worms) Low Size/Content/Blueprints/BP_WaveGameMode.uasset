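; Wave survival game mode that spawns enemies in waves and returns to the Lobby level once all players die.
; BeginPlay counts BP_TopDownCharacter players and binds their death events, calling NewWaveStarted inside that per-player loop.
; Each wave spawns CurrentWave × Difficulty BP_AICharacters at random points within fixed bounds, then binds their death events.
; Enemy deaths raise Score, fire OnEnemyDead and start the next wave when none remain.
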(event `self.ReceiveBeginPlay`
  ;[1 1 1] Setup beginning, by counting all players and adding it to remaining players, then bind the player death to notify us when one dies
  (`KismetSystemLibrary.Delay` 2.0)
  (`GameplayStatics.SetGamePaused` true)
  (bind _outactors (`GameplayStatics.GetAllActorsOfClass` "/Game/Blueprints/BP_TopDownCharacter.BP_TopDownCharacter_C"))
  (for _array_element _outactors
    (add `/Game/Blueprints/BP_TopDownCharacter.On Player Death` _array_element (delegate `On Player Death`))
    (`/Engine/EditorBlueprintResources/StandardMacros.IncrementInt` (`self.Remaining Players`)
      (:`  `
        (`GameplayStatics.SetGamePaused` false)
        (`self.NewWaveStarted`)))))

(event `On Player Death`
  (bind _remaining_players (`self.Remaining Players`))
  ;[1 1 1] Setup beginning, by counting all players and adding it to remaining players, then bind the player death to notify us when one dies
  (`/Engine/EditorBlueprintResources/StandardMacros.DecrementInt` _remaining_players
    (:`  `
      (if (not (`KismetMathLibrary.Conv_IntToBool` _remaining_players))
        (`GameplayStatics.OpenLevel` "Lobby")))))

(event `DecreaseEnemyCount`
  ;[1 1 1] This event occurs whenever an enemy dies and checks whether there are any left alive
  (bind _result (`/Engine/EditorBlueprintResources/StandardMacros.DecrementInt` (`self.AliveEnemies`))
    (:`  `
      (`/Engine/EditorBlueprintResources/StandardMacros.IncrementInt` (`self.Score`)
        (:`  `
          (`self.OnEnemyDead`)
          (if (not (`KismetMathLibrary.Conv_IntToBool` _result))
            (`self.NewWaveStarted`)))))))

(event `NewWaveStarted`
  ;[1 1 1] Occurs when a new wave starts, has to recount how many enemies are alive, and the delay is to make sure it doesnt run before all enemies are done spawning, the enemy on death event also needs to be rebound as they are new instances
  (`KismetSystemLibrary.Delay` 1.0)
  (`/Engine/EditorBlueprintResources/StandardMacros.IncrementInt` (`self.CurrentWave`)
    (:`  `
      (`self.CalculateEnemeis`)
      (`self.SpawnEnemies`)
      (bind _outactors (`GameplayStatics.GetAllActorsOfClass` "/Game/Blueprints/BP_AICharacter.BP_AICharacter_C"))
      (set `self.AliveEnemies` (`KismetArrayLibrary.Array_Length` _outactors))
      (for _array_element _outactors
        (add `/Game/Blueprints/BP_AICharacter.OnDeath` _array_element (delegate `DecreaseEnemyCount`))
        (`self.OnNewWaveStart`)))))

(fn `CalculateEnemeis`
  ;[1 1 1] Just as simple as doubling amount of enemies for each wave
  (set `self.EnemiesToSpawn` (* (`self.CurrentWave`) (`self.Difficulty`))))

(fn `OnRep_CurrentWave`)

(fn `SpawnEnemies`
  ;[1 1 1] Currently spawn enemies in a random location within a manually created range
  (for _ (range 1 (+ (`self.EnemiesToSpawn`) 1))
    (`|SpawnActorFromClass` "/Game/Blueprints/BP_AICharacter.BP_AICharacter_C" (`KismetMathLibrary.MakeTransform` (`KismetMathLibrary.MakeVector` (`KismetMathLibrary.RandomFloatInRange` -3800.0 3400.0) (`KismetMathLibrary.RandomFloatInRange` -7700.0) 189.0)) "AdjustIfPossibleButAlwaysSpawn" "MultiplyWithRoot" null null)))

(fn `StartWave`
  (`self.SpawnEnemies`))

(fn `UserConstructionScript`)