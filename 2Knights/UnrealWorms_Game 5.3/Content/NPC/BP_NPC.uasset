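; Melee enemy NPC that chases and attacks the player, feeding its AI blackboard sight, attack-range and death flags.
; AttackPlayer plays a montage and sphere-traces at the right hand to damage the player.
; TakeDamage triggers a random hit reaction with brief invulnerability against repeat hits from one swing.
; At zero health it stops movement, plays a death montage, destroys itself and fires the game mode's enemy-killed dispatcher.
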(event `self.PawnSensing.OnSeePawn`
  (params (Pawn :type "Pawn Object Reference"))
  ;[1 1 1] Has Enemy Seen Player? (Chase State)
  (cast `/Game/ThirdPerson/Blueprints/BP_ThirdPersonCharacter` Pawn)
  (`BlackboardComponent.SetValueAsBool` (`AIBlueprintHelperLibrary.GetBlackboard` (`AIBlueprintHelperLibrary.GetAIController` self)) "HasSeenPlayer" true))

(event `self.ReceiveTick`
  (params (DeltaSeconds :type "Float (single-precision)"))
  ;[1 1 1] Is Enemy In Range to Attack (Attack State)
  (`BlackboardComponent.SetValueAsBool` (`AIBlueprintHelperLibrary.GetBlackboard` (`AIBlueprintHelperLibrary.GetAIController` self)) "InRange" (< (`self.GetDistanceTo` (`GameplayStatics.GetPlayerCharacter` 0)) 100.0)))

(event `Event Hit React`
  ;[1 1 1] Enemy Animations
  ;;[1 1 1] Ractiion Animation
  (set `self.Can Be Damaged` false)
  (`|PlayMontage` (`self.Mesh`) (select `int` (`KismetMathLibrary.RandomIntegerInRange` 0 1) :`0` "/Game/Characters/Knight/Animations/Montages/sword_and_shield_impact__2__Montage.sword_and_shield_impact__2__Montage" :`1` "/Game/Characters/Knight/Animations/Montages/sword_and_shield_impact__3__Montage.sword_and_shield_impact__3__Montage" :!type "AnimMontage Object Reference")
    (:`then`
      (`GameplayStatics.PlaySound2D` "/Game/Audio/DamadgeSounds.DamadgeSounds" 1.0 1.0 0.0 null null)
      (`KismetSystemLibrary.Delay` 0.5))
    (:`OnCompleted`
      _))
  (set `self.Can Be Damaged` true))

(event `Event Death`
  ;[1 1 1] Enemy Animations
  ;;[1 1 1] Death Animation
  (`|PlayMontage` (`self.Mesh`) "/Game/Characters/Knight/Animations/Montages/sword_and_shield_death_Montage.sword_and_shield_death_Montage"
    (:`then`
      (`KismetSystemLibrary.Delay` 2.0)
      (`self.K2_DestroyActor`)
      (bind _outactors (`GameplayStatics.GetAllActorsOfClass` "/Game/ThirdPerson/Blueprints/BP_ThirdPersonGameMode.BP_ThirdPersonGameMode_C"))
      (`/Game/ThirdPerson/Blueprints/BP_ThirdPersonGameMode.EnemyKilledDispatcher` _outactors) ; Tells the Game Mode an\nenemy has been killed
    )))

(fn `attackanimation`)

(fn `AttackPlayer`
  (bind _returnvalue (`SceneComponent.GetSocketLocation` (`self.Mesh`) "RightHand"))
  (if (not (`self.IsDead`))
    (`self.PlayAnimMontage` "/Game/Characters/Knight/Animations/Montages/AM_Attack_1.AM_Attack_1")
    (bind (_outhit _returnvalue_2) (`KismetSystemLibrary.SphereTraceSingleForObjects` _returnvalue _returnvalue 100.0 (`|MakeArray` "ObjectTypeQuery3" :!type "EObjectTypeQuery Enum") false (`self.Out Actors`))) ; Same concept as the player's attack function
    (if _returnvalue_2
      (bind _asbp_third_person_character (cast `/Game/ThirdPerson/Blueprints/BP_ThirdPersonCharacter` (`.HitActor` (`GameplayStatics.BreakHitResult` _outhit))))
      (`/Game/ThirdPerson/Blueprints/BP_ThirdPersonCharacter.Take Damage` _asbp_third_person_character (`self.Damage`) (`self.GetActorForwardVector` (`self.GetOwner`))) ; calls the players Take damage function
    )))

(fn `TakeDamage`
  (params (Damage :type Integer))
  (if (`self.Can Be Damaged`)
    (`self.Event Hit React`)
    (bind _output_get (set `self.Health` (`KismetMathLibrary.Max` (- (`self.Health`) Damage))))
    (if (<= _output_get 0)
      (set `self.IsDead` true)
      (`MovementComponent.StopMovementImmediately` (`self.CharacterMovement`)) ; prevent the AI to move when it's effectively dead
      (`BlackboardComponent.SetValueAsBool` (`AIBlueprintHelperLibrary.GetBlackboard` (`AIBlueprintHelperLibrary.GetAIController` self)) "IsDead" (`self.IsDead`))
      (`self.Event Death`))))

(fn `UserConstructionScript`)